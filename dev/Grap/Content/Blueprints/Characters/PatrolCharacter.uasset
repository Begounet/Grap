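; PatrolCharacter is an AI-driven character Blueprint that supplies navigation data to its RandomWalkerAI controller.
; On BeginPlay, InitializeAI fetches the controller's Blackboard and writes the character's NavData object into the key named by BBKeyNavData.
; Helper functions return the typed AI controller and the mesh's ABP_Popuko animation instance through casts.
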(event `self.ReceiveBeginPlay`
  (`self.InitializeAI`))

(fn `GetABP`
  (returns (ABP :type "/Game/Meshes/Popuko/Animations/ABP_Popuko Object Reference"))
  (bind _asabp_popuko (cast `/Game/Meshes/Popuko/Animations/ABP_Popuko` (`SkeletalMeshComponent.GetAnimInstance` (`self.Mesh`)))
    (:`then`
      _)
    (:`CastFailed`
      _))
  (return _asabp_popuko))

(fn `GetAI`
  (returns (AI :type "/Game/Blueprints/AI/RandomWalkerAI Object Reference"))
  (bind _asrandom_walker_ai (cast `/Game/Blueprints/AI/RandomWalkerAI` (`AIBlueprintHelperLibrary.GetAIController` self))
    (:`then`
      _)
    (:`CastFailed`
      _))
  (return _asrandom_walker_ai))

(fn `InitializeAI`
  (`BlackboardComponent.SetValueAsObject` (`AIBlueprintHelperLibrary.GetBlackboard` (`self.GetAI`)) (`self.BBKey_NavData`) (`self.NavData`)))

(fn `UserConstructionScript`
  (`parent.UserConstructionScript`))