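; Pokupo character Blueprint for an AI-controlled wanderer that dies when it receives a shot.
; On BeginPlay it writes its NavData object into the blackboard of its AI_Wanderer controller.
; On a received shot it runs the parent handler, then calls Kill on both its ABP_Popuko animation Blueprint and the AI controller.
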(event `self.ReceiveBeginPlay`
  (`self.InitializeAI`))

(event `self.OnReceivedShot`
  (params (Hit :type "HitResult Structure"))
  (`parent.OnReceivedShot` Hit)
  (`/Game/Meshes/Popuko/Animations/ABP_Popuko.Kill` (`self.GetABP`))
  (`self.NotifyAI_Kill`))

(fn `GetABP`
  (returns (ABP :type "/Game/Meshes/Popuko/Animations/ABP_Popuko Object Reference"))
  (bind _asabp_popuko (cast `/Game/Meshes/Popuko/Animations/ABP_Popuko` (`SkeletalMeshComponent.GetAnimInstance` (`self.Mesh`)))
    (:`then`
      _)
    (:`CastFailed`
      _))
  (return _asabp_popuko))

(fn `GetAI`
  (returns (AI :type "/Game/Blueprints/AI/Wanderer/AI_Wanderer Object Reference"))
  (bind _asai_wanderer (cast `/Game/Blueprints/AI/Wanderer/AI_Wanderer` (`AIBlueprintHelperLibrary.GetAIController` self))
    (:`then`
      _)
    (:`CastFailed`
      _))
  (return _asai_wanderer))

(fn `InitializeAI`
  (`BlackboardComponent.SetValueAsObject` (`AIBlueprintHelperLibrary.GetBlackboard` (`self.GetAI`)) (`self.BBKey_NavData`) (`self.NavData`)))

(fn `NotifyAI_Kill`
  (`/Game/Blueprints/AI/Wanderer/AI_Wanderer.Kill` (`self.GetAI`)))

(fn `UserConstructionScript`
  (`parent.UserConstructionScript`))