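; Base character Blueprint that ends the game when the character is shot while flagged as the target.
; The OnShoot event calls OnReceivedShot, which checks IsTheTarget and, if set, calls TriggerGameEnd.
; TriggerGameEnd forwards to the FirstPersonGameMode, obtained through a helper function that casts the current game mode.
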(event `/Game/Blueprints/Components/IShootable.OnShoot`
  (`self.OnReceivedShot`))

(fn `GetFPSGameMode`
  (returns (GameMode :type "/Game/Blueprints/FirstPersonGameMode Object Reference"))
  (bind _asfirst_person_game_mode (cast `/Game/Blueprints/FirstPersonGameMode` (`GameplayStatics.GetGameMode`))
    (:`then`
      _)
    (:`CastFailed`
      _))
  (return _asfirst_person_game_mode))

(fn `OnReceivedShot`
  (if (`self.IsTheTarget`)
    (`self.TriggerGameEnd`)))

(fn `TriggerGameEnd`
  (`/Game/Blueprints/FirstPersonGameMode.TriggerGameEnd` (`self.GetFPSGameMode`)))

(fn `UserConstructionScript`)