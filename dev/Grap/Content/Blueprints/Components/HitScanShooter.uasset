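; Scene component that fires hitscan shots along its forward vector, limited by a cooldown timer that counts down on Tick.
; Shoot runs a line trace by collision profile out to the shoot distance once the cooldown has elapsed, then restarts the cooldown.
; On a hit it spawns an impact emitter and sends an OnShoot message to both the hit actor and the hit component, leaving the response to them.
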(event `self.ReceiveTick`
  (params (DeltaSeconds :type "Float (single-precision)"))
  (`self.UpdateCooldown` DeltaSeconds))

(fn `CanShoot`
  (returns (CanShoot :type Boolean))
  (return (`KismetMathLibrary.NearlyEqual_FloatFloat` (`self.CooldownRemaining`))))

(fn `InitCooldown`
  (set `self.CooldownRemaining` (`self.Cooldown`)))

(fn `Shoot`
  (bind _returnvalue (`self.K2_GetComponentLocation`))
  (if (`self.CanShoot`)
    (`self.InitCooldown`)
    (bind (_outhit _returnvalue_2) (`KismetSystemLibrary.LineTraceSingleByProfile` _returnvalue (+ _returnvalue (* (`KismetMathLibrary.GetForwardVector` (`self.K2_GetComponentRotation`)) (`self.ShootDistance`))) (`self.CollisionProfileName`)))
    (if _returnvalue_2
      (bind (_bblockinghit _binitialoverlap _time _distance _location _impactpoint _normal _impactnormal _physmat _hitactor _hitcomponent) (`GameplayStatics.BreakHitResult` _outhit))
      (`self.SpawnImpactFX` _impactpoint)
      (message `/Game/Blueprints/Components/IShootable.OnShoot` _hitactor _outhit)
      (message `/Game/Blueprints/Components/IShootable.OnShoot` _hitcomponent _outhit))))

(fn `SpawnImpactFX`
  (params (Location :type "Vector Structure"))
  (`GameplayStatics.SpawnEmitterAtLocation` (`self.ImpactFX`) Location))

(fn `UpdateCooldown`
  (params (DeltaSeconds :type "Float (double-precision)"))
  (set `self.CooldownRemaining` (`KismetMathLibrary.FMax` (- (`self.CooldownRemaining`) DeltaSeconds))))