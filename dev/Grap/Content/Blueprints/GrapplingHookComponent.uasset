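; Grappling hook component that pulls the player character toward a world object hit by a camera line trace.
; Setup supplies its references and tuning, then StartHook traces and launches the character toward the hit, once or repeatedly through a timer-polled gate when ProgressiveHook is set.
; A second looping timer interpolates the visible rope's location while its gate is open.
; Climb adds an upward launch while hooking against non-simulating components.
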(event `self.ReceiveBeginPlay`
  ;[1 1 1] Timers
  (if (`self.ProgressiveHook`)
    (`KismetSystemLibrary.K2_SetTimer` null "Object" 0.15 true))
  (`KismetSystemLibrary.K2_SetTimer` null "Rope" 0.15 true))

(event `Object`
  (bind _playercharacter (`self.PlayerCharacter`))
  ;[1 1 1] Jump to Hooked Object
  (bind _returnvalue (- (stale `HookObject` HitLocation) (`Actor.K2_GetActorLocation` (`GameplayStatics.GetPlayerPawn` 0))))
  (if (>= (`KismetMathLibrary.VSize` _returnvalue) (`self.HookPadding`))
    (`/Engine/EditorBlueprintResources/StandardMacros.Gate` true :!label _label
      (:`Exit`
        (bind _returnvalue_2 (* _returnvalue (`self.HookSpeedMultiplier`)))
        (`self.ShowHook` _returnvalue_2 :!label _label_2)
        (`Character.LaunchCharacter` _playercharacter (0.0 0.0 -500.0) true true)
        (`KismetSystemLibrary.Delay` 0.2)
        (`Character.LaunchCharacter` _playercharacter _returnvalue_2 false false)
        (`KismetSystemLibrary.Delay` 0.4)
        (`self.HideHook`)))
    (else
      (goto _label :!via `Close`))))

(event `HookObject`
  (params (HitLocation :type "Vector Structure"))
  ;[1 1 1] Jump to Hooked Object
  (if (`self.ProgressiveHook`)
    (goto _label :!via `Open`)
    (else
      (goto _label_2))))

(event `Close Object`
  ;[1 1 1] Jump to Hooked Object
  (goto _label :!via `Close`))

(event `Rope`
  ;[1 1 1] Show Hook
  (`/Engine/EditorBlueprintResources/StandardMacros.Gate` true :!label _label_3
    (:`Exit`
      (`self.K2_SetWorldLocation` (`self.GrapplingRope`) (`KismetMathLibrary.VInterpTo` (`self.K2_GetComponentLocation` (`self.GrapplingRope`)) (stale `ShowHook` HitLocation) (`KismetSystemLibrary.K2_GetTimerElapsedTime` null "Rope") 1.0) false false))))

(event `ShowHook`
  (params (HitLocation :type "Vector Structure"))
  ;[1 1 1] Show Hook
  (`self.SetVisibility` (`self.GrapplingRope`) true false)
  (goto _label_3 :!via `Open`))

(event `Close Rope`
  ;[1 1 1] Show Hook
  (goto _label_3 :!via `Close`))

(event `HideHook`
  (`self.SetVisibility` (`self.GrapplingRope`) false false)
  (set `self.IsHooking` false))

(fn `Climb`
  (params (Other :type "PrimitiveComponent Object Reference"))
  (if (`self.IsSimulatingPhysics` Other "None")
    _
    (elif (`self.IsHooking`)
      (`Character.LaunchCharacter` (`self.PlayerCharacter`) (0.0 0.0 400.0) false false))))

(fn `Setup`
  (params (CameraComponent :type "CameraComponent Object Reference") (PlayerCharacter :type "/Game/Blueprints/FirstPersonCharacter Object Reference") (MaxHookDistance :type "Float (double-precision)" :default 5000.0) (HookPadding :type "Float (double-precision)" :default 125.0) (HookSpeedMultiplier :type "Float (double-precision)" :default 2.5) (ProgressiveHook :type Boolean) (GrapplingRope :type "CableComponent Object Reference"))
  (`|ExecutionSequence`
    (:`then_0`
      (set `self.CameraComponent` CameraComponent))
    (:`then_1`
      (set `self.PlayerCharacter` PlayerCharacter))
    (:`then_2`
      (set `self.MaxHookDistance` MaxHookDistance))
    (:`then_3`
      (set `self.HookPadding` HookPadding))
    (:`then_4`
      (set `self.HookSpeedMultiplier` HookSpeedMultiplier))
    (:`then_5`
      (set `self.ProgressiveHook` ProgressiveHook))
    (:`then_6`
      (set `self.GrapplingRope` GrapplingRope))))

(fn `StartHook`
  (bind _cameracomponent (`self.CameraComponent`))
  (bind _returnvalue (`self.K2_GetComponentLocation` _cameracomponent))
  ;[1 1 1] Run Trace for Objects
  (set `self.IsHooking` true)
  (bind (_outhit _returnvalue_2) (`KismetSystemLibrary.LineTraceSingleForObjects` :`Start` _returnvalue :`End` (+ _returnvalue (`KismetMathLibrary.GreaterGreater_VectorRotator` (`KismetMathLibrary.MakeVector` (`self.MaxHookDistance`)) (`self.K2_GetComponentRotation` _cameracomponent))) :`ObjectTypes` (`|MakeArray` "ObjectTypeQuery1" "ObjectTypeQuery2" :!type "EObjectTypeQuery Enum") :`DrawDebugType` "Persistent"))
  (if _returnvalue_2
    (`self.HookObject` (`.Location` (`GameplayStatics.BreakHitResult` _outhit)))
    (else
      (`self.HideHook`))))

(fn `StopHook`
  (`self.Close Object`))